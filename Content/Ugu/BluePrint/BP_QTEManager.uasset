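; Quick-time event manager that runs four scripted QTEs, where failure calls PlayerDeath on the first-person character.
; Start_QTE swaps character input for its own and opens a Delay-timed window, which the AnyKey handler judges through shared state flags.
; QTEs 1-2 add cameras, cinematics, slow motion and BP_CrabiCrabobo trigger resets.
; QTE 3 chains E-mashing into a left click that grants the knife; QTE 4 is one randomly delayed press.
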(event `Key|AnyKey`
  (params (Key :type "Key Structure"))
  (bind _returnvalue (`GameplayStatics.GetPlayerController` 0))
  (bind _as_bp_first_person_character (`self.As BP First Person Character`))
  (:`Pressed`
    (switch `int` (`self.QTE ID`)
      (:`1`
        ; QTE1&2
        (if (and (`self.IsQTEActive`) (`self.CanPress`) (== Key (`self.QTEKey`))) :!label _label
          (`GameplayStatics.SetGlobalTimeDilation` 1.0)
          (`KismetSystemLibrary.PrintString` "Succes")
          (`SceneComponent.K2_SetWorldLocation` (`Actor.RootComponent` (`GameplayStatics.GetPlayerCharacter` 0)) (`self.K2_GetActorLocation` (`self.LocationPlayerAfterQTE`)) false true)
          (`PlayerController.SetViewTargetWithBlend` (`GameplayStatics.GetPlayerController` 0) (`GameplayStatics.GetPlayerCharacter` 0) 0.0 "VTBlend_Linear" 3.0 false)
          (set `self.QTESuccess` true)
          (set `self.IsQTEActive` false)
          (set `self.CanPress` false)
          (`self.EnableInput` (`GameplayStatics.GetPlayerCharacter` 0) (`GameplayStatics.GetPlayerController` 0))
          (`self.DisableInput` (`GameplayStatics.GetPlayerController` 0))
          (if (`self.bIsDelatable`)
            (`/Game/Ugu/BluePrint/BP_CrabiCrabobo.Destroy_Actor` (`self.ActorQTE1-2`))
            (else
              (`KismetSystemLibrary.Delay` (`self.delay`))
              (bind _asbp_crabi_crabobo (cast `/Game/Ugu/BluePrint/BP_CrabiCrabobo` (`self.CurrentActor_QTE`)))
              (`/Game/Ugu/BluePrint/BP_CrabiCrabobo.ResetQTETrigger` _asbp_crabi_crabobo)))
          (else
            (`GameplayStatics.SetGlobalTimeDilation` 1.0)
            (set `self.QTESuccess` false)
            (set `self.IsQTEActive` false)
            (set `self.CanPress` false)
            (set `self.T'es deja trompé` true)
            (`KismetSystemLibrary.PrintString` "UGU")
            (`SceneComponent.K2_SetWorldLocation` (`Actor.RootComponent` (`GameplayStatics.GetPlayerCharacter` 0)) (`self.K2_GetActorLocation` (`self.LocationPlayerAfterQTE`)) false true)
            (`PlayerController.SetViewTargetWithBlend` (`GameplayStatics.GetPlayerController` 0) (`GameplayStatics.GetPlayerCharacter` 0) 0.0 "VTBlend_Linear" 3.0 false)
            (bind (_outactor _returnvalue_2) (`LevelSequencePlayer.CreateLevelSequencePlayer` (`self.Cinematic1Loose`)))
            (`MovieSceneSequencePlayer.Play` _returnvalue_2)
            (`self.EnableInput` (`GameplayStatics.GetPlayerCharacter` 0) _returnvalue)
            (`self.DisableInput` _returnvalue)
            (`/Game/Ugu/FirstPerson/Blueprints/BP_FirstPersonCharacter.PlayerDeath` (`self.As BP First Person Character`))
            (`KismetSystemLibrary.Delay` (`self.delay`))
            (bind _asbp_crabi_crabobo_2 (cast `/Game/Ugu/BluePrint/BP_CrabiCrabobo` (`self.CurrentActor_QTE`)))
            (`/Game/Ugu/BluePrint/BP_CrabiCrabobo.ResetQTETrigger` _asbp_crabi_crabobo_2))))
      (:`2`
        (goto _label))
      (:`3`
        ; QTE3
        (if (== Key (`self.QTEKey`))
          (if (and (`self.IsQTEActive`) (`self.CanPress`))
            (if (`self.bCanValidate`)
              (`KismetSystemLibrary.PrintString` "Succes")
              (set `self.QTESuccess` true)
              (set `self.IsQTEActive` false)
              (set `self.CanPress` false)
              (`self.EnableInput` (`GameplayStatics.GetPlayerCharacter` 0) (`GameplayStatics.GetPlayerController` 0))
              (`self.DisableInput` (`GameplayStatics.GetPlayerController` 0))
              (if (`self.bIsDelatable`)
                (set `/Game/Ugu/FirstPerson/Blueprints/BP_FirstPersonCharacter.KnifeLunch?` true _as_bp_first_person_character)
                (set `/Game/Ugu/FirstPerson/Blueprints/BP_FirstPersonCharacter.Knife?` true _as_bp_first_person_character)
                (`self.K2_DestroyActor` (`self.CurrentActor_QTE`)))
              (else
                (bind _output_get (set `self.MashCount` (+ (`self.MashCount`) 1)))
                (`KismetSystemLibrary.PrintString` (`KismetStringLibrary.Conv_IntToString` _output_get))
                (if (>= (`self.MashCount`) (`self.MashRequired`))
                  (`self.DisableInput` (`GameplayStatics.GetPlayerController` 0))
                  (set `self.bCanValidate` true)
                  (set `self.IsQTEActive` false)
                  (set `self.CanPress` false))))
            (else
              (`KismetSystemLibrary.PrintString` "Fail")
              (set `self.QTESuccess` false)
              (set `self.IsQTEActive` false)
              (set `self.CanPress` false)
              (`self.EnableInput` (`GameplayStatics.GetPlayerCharacter` 0) (`GameplayStatics.GetPlayerController` 0))
              (`self.DisableInput` (`GameplayStatics.GetPlayerController` 0))
              (`/Game/Ugu/FirstPerson/Blueprints/BP_FirstPersonCharacter.PlayerDeath` (`self.As BP First Person Character`))))))
      (:`4`
        ; QTE4
        (if (== Key (`self.QTEKey`))
          (if (and (`self.IsQTEActive`) (`self.CanPress`))
            (`KismetSystemLibrary.PrintString` "Succes")
            (set `self.QTESuccess` true)
            (set `self.IsQTEActive` false)
            (set `self.CanPress` false)
            (`self.EnableInput` (`GameplayStatics.GetPlayerCharacter` 0) (`GameplayStatics.GetPlayerController` 0))
            (`self.DisableInput` (`GameplayStatics.GetPlayerController` 0))
            (else
              (`KismetSystemLibrary.PrintString` "Fail")
              (set `self.QTESuccess` false)
              (set `self.IsQTEActive` false)
              (set `self.CanPress` false)
              (`self.EnableInput` (`GameplayStatics.GetPlayerCharacter` 0) (`GameplayStatics.GetPlayerController` 0))
              (`self.DisableInput` (`GameplayStatics.GetPlayerController` 0))
              (`/Game/Ugu/FirstPerson/Blueprints/BP_FirstPersonCharacter.PlayerDeath` (`self.As BP First Person Character`)))))))))

(event `CameraQTE`
  (bind _returnvalue (`self.K2_GetActorLocation` (`GameplayStatics.GetPlayerCharacter` 0)))
  (bind _returnvalue_2 (`|SpawnActorFromClass` "/Game/Ugu/BluePrint/BP_Camera_QTE.BP_Camera_QTE_C" (`KismetMathLibrary.MakeTransform` _returnvalue (`KismetMathLibrary.Conv_VectorToRotator` _returnvalue)) "Undefined" "MultiplyWithRoot" null null)))

(event `CameraQTE2`
  (bind _returnvalue (`self.K2_GetActorLocation` (`GameplayStatics.GetPlayerCharacter` 0)))
  (bind _returnvalue_2 (`|SpawnActorFromClass` "/Game/Ugu/BluePrint/BP_Camera_QTE.BP_Camera_QTE_C" (`KismetMathLibrary.MakeTransform` _returnvalue (`KismetMathLibrary.Conv_VectorToRotator` _returnvalue)) "Undefined" "MultiplyWithRoot" null null))
  (`self.K2_SetActorLocationAndRotation` _returnvalue_2 _returnvalue (struct :`Pitch` -20.0) false false)
  (`PlayerController.SetViewTargetWithBlend` (`GameplayStatics.GetPlayerController` 0) _returnvalue_2 1.0 "VTBlend_Linear" 3.0 false))

(event `self.ReceiveBeginPlay`
  (`self.DisableInput` (`GameplayStatics.GetPlayerController` 0)))

(event `Start_QTE`
  (params (QTE_ID :type Integer) (CurrentActor :type "Actor Object Reference"))
  (bind _returnvalue (`GameplayStatics.GetPlayerController` 0))
  (bind _returnvalue_2 (`GameplayStatics.GetPlayerController` 0))
  (bind _returnvalue_3 (`GameplayStatics.GetPlayerController` 0))
  (bind _returnvalue_4 (`GameplayStatics.GetPlayerCharacter` 0))
  (bind _returnvalue_5 (`GameplayStatics.GetPlayerController` 0))
  (bind _qtetimewindow (`self.QTETimeWindow`))
  (bind _bcanvalidate (`self.bCanValidate`))
  (bind _qtetimewindow_2 (`self.QTETimeWindow`))
  (bind _qtetimewindow_3 (`self.QTETimeWindow`))
  (bind _qtetimewindow_4 (`self.QTETimeWindow`))
  (bind _qtetimewindow_5 (`self.QTETimeWindow`))
  (bind _returnvalue_6 (`self.K2_GetActorLocation` (`self.LocationPlayerAfterQTE`)))
  (bind _rootcomponent (`Actor.RootComponent` (`GameplayStatics.GetPlayerCharacter` 0)))
  (bind _output_get (set `self.QTE ID` QTE_ID))
  (set `self.CurrentActor_QTE` CurrentActor)
  (bind _asbp_first_person_character (cast `/Game/Ugu/FirstPerson/Blueprints/BP_FirstPersonCharacter` (`GameplayStatics.GetPlayerCharacter` 0)))
  (set `self.As BP First Person Character` _asbp_first_person_character)
  (set `self.IsQTEActive` true)
  (set `self.CanPress` false)
  (switch `int` _output_get
    (:`1`
      ; QTE1
      (`PlayerController.SetViewTargetWithBlend` (`GameplayStatics.GetPlayerController` 0) (`self.REF_Camera1&2`) 1.0 "VTBlend_Linear" 3.0 false)
      (bind (_outactor _returnvalue_7) (`LevelSequencePlayer.CreateLevelSequencePlayer` (`self.Cinematic1Generic`)))
      (`MovieSceneSequencePlayer.Play` _returnvalue_7)
      (`KismetSystemLibrary.PrintString` "QTE 1")
      (set `self.bIsDelatable` true)
      (`self.DisableInput` (`GameplayStatics.GetPlayerCharacter` 0) (`GameplayStatics.GetPlayerController` 0))
      (set `self.QTEKey` "E")
      (set `self.QTETimeWindow` 0.5)
      (`KismetSystemLibrary.Delay` 1.5)
      (`self.EnableInput` (`GameplayStatics.GetPlayerController` 0))
      (set `self.CanPress` true)
      (`GameplayStatics.SetGlobalTimeDilation` 0.2)
      (`KismetSystemLibrary.PrintString` "Appuyer sur E" true true (struct :`R` 0.322075 :`G` 1.0 :`B` 0.659893 :`A` 1.0) _qtetimewindow_4)
      (`KismetSystemLibrary.Delay` _qtetimewindow_4)
      (if (`self.QTESuccess`)
        (`GameplayStatics.SetGlobalTimeDilation` 1.0)
        (`KismetSystemLibrary.PrintString` "C'est gagné")
        (set `self.IsQTEActive` false)
        (set `self.CanPress` false)
        (`self.DisableInput` (`GameplayStatics.GetPlayerController` 0))
        (`self.EnableInput` _returnvalue_4 _returnvalue_3)
        (`PlayerController.SetViewTargetWithBlend` _returnvalue_3 _returnvalue_4 1.0 "VTBlend_Linear" 3.0 false)
        (`KismetSystemLibrary.Delay` (`self.delay`))
        (bind _asbp_crabi_crabobo (cast `/Game/Ugu/BluePrint/BP_CrabiCrabobo` (`self.CurrentActor_QTE`)))
        (`/Game/Ugu/BluePrint/BP_CrabiCrabobo.ResetQTETrigger` _asbp_crabi_crabobo)
        (else
          (`KismetSystemLibrary.PrintString` "Fail")
          (`KismetSystemLibrary.Delay` 1.0)
          (if (not (`self.T'es deja trompé`))
            (`GameplayStatics.SetGlobalTimeDilation` 1.0)
            (`SceneComponent.K2_SetWorldLocation` (`Actor.RootComponent` (`GameplayStatics.GetPlayerController` 0)) (`self.K2_GetActorLocation` (`self.LocationPlayerAfterQTE`)) false false)
            (`PlayerController.SetViewTargetWithBlend` (`GameplayStatics.GetPlayerController` 0) (`GameplayStatics.GetPlayerCharacter` 0) 0.0 "VTBlend_Linear" 3.0 false)
            (bind (_outactor_2 _returnvalue_8) (`LevelSequencePlayer.CreateLevelSequencePlayer` (`self.Cinematic1Loose`)))
            (`MovieSceneSequencePlayer.Play` _returnvalue_8)
            (set `self.IsQTEActive` false)
            (set `self.CanPress` false)
            (`self.DisableInput` (`GameplayStatics.GetPlayerController` 0))
            (`self.EnableInput` (`GameplayStatics.GetPlayerCharacter` 0) (`GameplayStatics.GetPlayerController` 0))
            (`/Game/Ugu/FirstPerson/Blueprints/BP_FirstPersonCharacter.PlayerDeath` (`self.As BP First Person Character`))
            (`KismetSystemLibrary.Delay` (`self.delay`))
            (bind _asbp_crabi_crabobo_2 (cast `/Game/Ugu/BluePrint/BP_CrabiCrabobo` (`self.CurrentActor_QTE`)))
            (`/Game/Ugu/BluePrint/BP_CrabiCrabobo.ResetQTETrigger` _asbp_crabi_crabobo_2)))))
    (:`2`
      ; QTE2
      (`PlayerController.SetViewTargetWithBlend` (`GameplayStatics.GetPlayerController` 0) (`self.REF_Camera1&2`) 1.0 "VTBlend_Linear" 3.0 false)
      (bind (_outactor_3 _returnvalue_9) (`LevelSequencePlayer.CreateLevelSequencePlayer` (`self.Cinematic1Generic`)))
      (`MovieSceneSequencePlayer.Play` _returnvalue_9)
      (`KismetSystemLibrary.PrintString` "QTE 2")
      (`self.DisableInput` (`GameplayStatics.GetPlayerCharacter` 0) (`GameplayStatics.GetPlayerController` 0))
      (set `self.QTEKey` "E")
      (set `self.QTETimeWindow` 1.0)
      (`KismetSystemLibrary.Delay` 1.5)
      (`self.EnableInput` (`GameplayStatics.GetPlayerController` 0))
      (set `self.CanPress` true)
      (`GameplayStatics.SetGlobalTimeDilation` 0.2)
      (`KismetSystemLibrary.PrintString` "Appuyer sur E" true true (struct :`R` 0.322075 :`G` 1.0 :`B` 0.659893 :`A` 1.0) _qtetimewindow)
      (`KismetSystemLibrary.Delay` _qtetimewindow)
      (if (`self.QTESuccess`)
        (`GameplayStatics.SetGlobalTimeDilation` 1.0)
        (`KismetSystemLibrary.PrintString` "C'est gagné")
        (`SceneComponent.K2_SetWorldLocation` _rootcomponent _returnvalue_6 false false)
        (`PlayerController.SetViewTargetWithBlend` (`GameplayStatics.GetPlayerController` 0) (`GameplayStatics.GetPlayerCharacter` 0) 1.0 "VTBlend_Linear" 3.0 false)
        (set `self.IsQTEActive` false)
        (set `self.CanPress` false)
        (`self.DisableInput` _returnvalue)
        (`self.EnableInput` (`GameplayStatics.GetPlayerCharacter` 0) _returnvalue)
        (`KismetSystemLibrary.Delay` (`self.delay`))
        (bind _asbp_crabi_crabobo_3 (cast `/Game/Ugu/BluePrint/BP_CrabiCrabobo` (`self.CurrentActor_QTE`)))
        (`/Game/Ugu/BluePrint/BP_CrabiCrabobo.ResetQTETrigger` _asbp_crabi_crabobo_3)
        (elif (not (`self.T'es deja trompé`))
          (`KismetSystemLibrary.PrintString` "Fail")
          (`GameplayStatics.SetGlobalTimeDilation` 1.0)
          (`SceneComponent.K2_SetWorldLocation` _rootcomponent _returnvalue_6 false false)
          (`PlayerController.SetViewTargetWithBlend` (`GameplayStatics.GetPlayerController` 0) (`GameplayStatics.GetPlayerCharacter` 0) 1.0 "VTBlend_Linear" 3.0 false)
          (bind (_outactor_4 _returnvalue_10) (`LevelSequencePlayer.CreateLevelSequencePlayer` (`self.Cinematic1Loose`)))
          (`MovieSceneSequencePlayer.Play` _returnvalue_10)
          (set `self.QTESuccess` false)
          (set `self.IsQTEActive` false)
          (set `self.CanPress` false)
          (set `self.bCanValidate` false)
          (`self.DisableInput` _returnvalue_2)
          (`self.EnableInput` (`GameplayStatics.GetPlayerCharacter` 0) _returnvalue_2)
          (`/Game/Ugu/FirstPerson/Blueprints/BP_FirstPersonCharacter.PlayerDeath` (`self.As BP First Person Character`))
          (`KismetSystemLibrary.Delay` (`self.delay`))
          (bind _asbp_crabi_crabobo_4 (cast `/Game/Ugu/BluePrint/BP_CrabiCrabobo` (`self.CurrentActor_QTE`)))
          (`/Game/Ugu/BluePrint/BP_CrabiCrabobo.ResetQTETrigger` _asbp_crabi_crabobo_4))))
    (:`3`
      ; QTE3
      (`KismetSystemLibrary.PrintString` "QTE 3")
      (set `self.bIsDelatable` true)
      (`self.DisableInput` (`GameplayStatics.GetPlayerCharacter` 0) (`GameplayStatics.GetPlayerController` 0))
      (set `self.QTEKey` "E")
      (set `self.QTETimeWindow` 2.0)
      (`KismetSystemLibrary.Delay` (`KismetMathLibrary.RandomFloatInRange` 1.0 3.0))
      (`self.EnableInput` (`GameplayStatics.GetPlayerController` 0))
      (set `self.IsQTEActive` true)
      (set `self.QTESuccess` false)
      (set `self.CanPress` true)
      (set `self.bCanValidate` false)
      (set `self.MashCount` 0)
      (set `self.MashRequired` 10)
      (`KismetSystemLibrary.PrintString` "Appuyer sur E" true true (struct :`R` 0.322075 :`G` 1.0 :`B` 0.659893 :`A` 1.0) _qtetimewindow_2)
      (`KismetSystemLibrary.Delay` _qtetimewindow_2)
      (`KismetSystemLibrary.PrintString` (`KismetStringLibrary.Conv_BoolToString` _bcanvalidate) true true (struct :`R` 0.322075 :`G` 1.0 :`B` 0.659893 :`A` 1.0))
      (if _bcanvalidate
        (`self.EnableInput` (`GameplayStatics.GetPlayerController` 0))
        (set `self.QTEKey` "LeftMouseButton")
        (set `self.QTETimeWindow` 1.0)
        (`KismetSystemLibrary.Delay` (`KismetMathLibrary.RandomFloatInRange` 1.0 3.0))
        (set `self.IsQTEActive` true)
        (set `self.CanPress` true)
        (`KismetSystemLibrary.PrintString` "Appuyer sur Click Gauche" true true (struct :`R` 0.322075 :`G` 1.0 :`B` 0.659893 :`A` 1.0) _qtetimewindow_3)
        (`KismetSystemLibrary.Delay` _qtetimewindow_3)
        (if (`self.IsQTEActive`)
          (`KismetSystemLibrary.PrintString` "Fail")
          (set `self.IsQTEActive` false)
          (set `self.CanPress` false)
          (`self.EnableInput` (`GameplayStatics.GetPlayerCharacter` 0) _returnvalue_5)
          (`self.DisableInput` _returnvalue_5)
          (`/Game/Ugu/FirstPerson/Blueprints/BP_FirstPersonCharacter.PlayerDeath` (`self.As BP First Person Character`)))
        (else
          (`KismetSystemLibrary.PrintString` "Fail")
          (set `self.IsQTEActive` false)
          (set `self.CanPress` false)
          (`self.EnableInput` (`GameplayStatics.GetPlayerCharacter` 0) (`GameplayStatics.GetPlayerController` 0))
          (`/Game/Ugu/FirstPerson/Blueprints/BP_FirstPersonCharacter.PlayerDeath` (`self.As BP First Person Character`)))))
    (:`4`
      ; QTE4
      (`KismetSystemLibrary.PrintString` "QTE4")
      (`self.DisableInput` (`GameplayStatics.GetPlayerCharacter` 0) (`GameplayStatics.GetPlayerController` 0))
      (set `self.QTEKey` "E")
      (set `self.QTETimeWindow` 1.0)
      (`KismetSystemLibrary.Delay` (`KismetMathLibrary.RandomFloatInRange` 1.0 3.0))
      (`self.EnableInput` (`GameplayStatics.GetPlayerController` 0))
      (set `self.CanPress` true)
      (`KismetSystemLibrary.PrintString` "Appuyer sur E" true true (struct :`R` 0.322075 :`G` 1.0 :`B` 0.659893 :`A` 1.0) _qtetimewindow_5)
      (`KismetSystemLibrary.Delay` _qtetimewindow_5)
      (if (`self.IsQTEActive`)
        (`KismetSystemLibrary.PrintString` "Fail")
        (set `self.IsQTEActive` false)
        (set `self.CanPress` false)
        (`self.DisableInput` (`GameplayStatics.GetPlayerController` 0))
        (`self.EnableInput` (`GameplayStatics.GetPlayerCharacter` 0) (`GameplayStatics.GetPlayerController` 0))
        (`/Game/Ugu/FirstPerson/Blueprints/BP_FirstPersonCharacter.PlayerDeath` (`self.As BP First Person Character`))))))

(fn `UserConstructionScript`)