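; BP_Crabivole_knife is a knife-thief crab actor that triggers a quick-time event when the first-person character touches it.
; It starts hidden without collision until CrabivoleurDeCouteau reveals it and enables its box.
; Player overlap disables further overlaps and starts QTE 3 through QTEManagerRef, while ResetQTECrabKnife re-arms the trigger.
; DestroyActorQTE3 dissolves five meshes with timeline-driven dynamic materials, then destroys the actor after a delay.
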(event `Destroy Actor QTE3`
  (bind _cube3 (`self.Cube3`))
  (bind _cube4 (`self.Cube4`))
  (bind _crabi1 (`self.Crabi1`))
  (bind _cube1 (`self.Cube1`))
  (bind _cube2 (`self.Cube2`))
  (set `PrimitiveComponent.bGenerateOverlapEvents` false (`self.Box`))
  (`|ExecutionSequence`
    (:`then_0`
      (bind _returnvalue (`PrimitiveComponent.CreateDynamicMaterialInstance` _crabi1 0 (`PrimitiveComponent.GetMaterial` _crabi1 0) "None"))
      (bind (_direction _newtrack_0) (`Timeline|Timeline` :!via `PlayFromStart`)
        (:`Update`
          (`MaterialInstanceDynamic.SetScalarParameterValue` _returnvalue "Disolve" _newtrack_0)
          (`KismetSystemLibrary.Delay` 3.0)
          (`self.K2_DestroyActor`))))
    (:`then_1`
      (bind _returnvalue_2 (`PrimitiveComponent.CreateDynamicMaterialInstance` _cube1 0 (`PrimitiveComponent.GetMaterial` _cube1 0) "None"))
      (bind (_direction_2 _newtrack_0_2) (`Timeline|Timeline_0` :!via `PlayFromStart`)
        (:`Update`
          (`MaterialInstanceDynamic.SetScalarParameterValue` _returnvalue_2 "Disolve" _newtrack_0_2)
          (`KismetSystemLibrary.Delay` 3.0)
          (`self.K2_DestroyActor`))))
    (:`then_2`
      (bind _returnvalue_3 (`PrimitiveComponent.CreateDynamicMaterialInstance` _cube2 0 (`PrimitiveComponent.GetMaterial` _cube2 0) "None"))
      (bind (_direction_3 _newtrack_0_3) (`Timeline|Timeline_1` :!via `PlayFromStart`)
        (:`Update`
          (`MaterialInstanceDynamic.SetScalarParameterValue` _returnvalue_3 "Disolve" _newtrack_0_3)
          (`KismetSystemLibrary.Delay` 3.0)
          (`self.K2_DestroyActor`))))
    (:`then_3`
      (bind _returnvalue_4 (`PrimitiveComponent.CreateDynamicMaterialInstance` _cube3 0 (`PrimitiveComponent.GetMaterial` _cube3 0) "None"))
      (bind (_direction_4 _newtrack_0_4) (`Timeline|Timeline_2` :!via `PlayFromStart`)
        (:`Update`
          (`MaterialInstanceDynamic.SetScalarParameterValue` _returnvalue_4 "Disolve" _newtrack_0_4)
          (`KismetSystemLibrary.Delay` 3.0)
          (`self.K2_DestroyActor`))))
    (:`then_4`
      (bind _returnvalue_5 (`PrimitiveComponent.CreateDynamicMaterialInstance` _cube4 0 (`PrimitiveComponent.GetMaterial` _cube4 0) "None"))
      (bind (_direction_5 _newtrack_0_5) (`Timeline|Timeline_3` :!via `PlayFromStart`)
        (:`Update`
          (`MaterialInstanceDynamic.SetScalarParameterValue` _returnvalue_5 "Disolve" _newtrack_0_5)
          (`KismetSystemLibrary.Delay` 3.0)
          (`self.K2_DestroyActor`))))))

(event `ResetQTECrabKnife`
  (set `PrimitiveComponent.bGenerateOverlapEvents` true (`self.Box`)))

(event `self.ReceiveBeginPlay`
  (`SceneComponent.SetVisibility` (`self.DefaultSceneRoot1`) false true)
  (`PrimitiveComponent.SetCollisionEnabled` (`self.Box`) "NoCollision"))

(event `CrabivoleurDeCouteau`
  (`SceneComponent.SetVisibility` (`self.DefaultSceneRoot1`) true true)
  (`PrimitiveComponent.SetCollisionEnabled` (`self.Box`) "QueryAndPhysics"))

(event `self.Box.OnComponentBeginOverlap`
  (params (OverlappedComponent :type "PrimitiveComponent Object Reference") (OtherActor :type "Actor Object Reference") (OtherComp :type "PrimitiveComponent Object Reference") (OtherBodyIndex :type Integer) (bFromSweep :type Boolean) (SweepResult :type "HitResult Structure (by ref)"))
  (bind _qtemanagerref (`self.QTEManagerRef`))
  (cast `/Game/Ugu/FirstPerson/Blueprints/BP_FirstPersonCharacter` OtherActor)
  (set `PrimitiveComponent.bGenerateOverlapEvents` false (`self.Box`))
  (set `self.QTE_ID` 3)
  (`/Engine/EditorBlueprintResources/StandardMacros.IsValid` _qtemanagerref
    (:`Is Valid`
      (`/Game/Ugu/BluePrint/BP_QTEManager.Start_QTE` _qtemanagerref (`self.QTE_ID`) self))))

(fn `UserConstructionScript`)