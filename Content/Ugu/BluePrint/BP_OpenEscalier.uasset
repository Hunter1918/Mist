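; Stairs actor that stays hidden and non-collidable until Open_Stairs reveals it with an aura and plays a cinematic.
; During the sequence it recalls the knife, locks player input and aiming, and switches to a cinematic camera.
; It then teleports and reorients the player, returns the view and shows the WBP_Cladigo widget, passing itself to it.
; RemoveUI clears the widget, hides the aura and restores input.
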(event `RemoveUI`
  (`KismetSystemLibrary.PrintString` "JAJAJAJAJA")
  (`Widget.RemoveFromParent` (`self.REF_UI`))
  (`PlayerController.SetViewTargetWithBlend` (`GameplayStatics.GetPlayerController` 0) (`GameplayStatics.GetPlayerCharacter` 0) 1.0 "VTBlend_Linear" 3.0 false)
  (`self.EnableInput` (`GameplayStatics.GetPlayerCharacter` 0) (`GameplayStatics.GetPlayerController` 0))
  (`SceneComponent.SetVisibility` (`self.BP_C_Aura`) false false)
  (set `/Game/Ugu/FirstPerson/Blueprints/BP_FirstPersonCharacter.bCanAIM` true (`self.As BP First Person Character`)))

(event `self.ReceiveBeginPlay`
  (`SceneComponent.SetVisibility` (`self.Stairs2`) false false)
  (`PrimitiveComponent.SetCollisionEnabled` (`self.Stairs2`) "NoCollision"))

(event `Open_Stairs`
  (bind _returnvalue (`GameplayStatics.GetPlayerController` 0))
  (bind _returnvalue_2 (`GameplayStatics.GetPlayerController` 0))
  (bind _returnvalue_3 (`GameplayStatics.GetPlayerCharacter` 0))
  (bind _returnvalue_4 (`GameplayStatics.GetPlayerCharacter` 0))
  (bind _returnvalue_5 (`GameplayStatics.GetPlayerCharacter` 0))
  (bind _as_bp_first_person_character (`self.As BP First Person Character`))
  (`SceneComponent.SetVisibility` (`self.Stairs2`) true false)
  (`SceneComponent.SetVisibility` (`self.BP_C_Aura`) true false)
  (`PrimitiveComponent.SetCollisionEnabled` (`self.Stairs2`) "QueryAndPhysics")
  (bind _asbp_first_person_character (cast `/Game/Ugu/FirstPerson/Blueprints/BP_FirstPersonCharacter` _returnvalue_4))
  (bind _output_get (set `self.As BP First Person Character` _asbp_first_person_character))
  (set `Pawn.bUseControllerRotationYaw` false _output_get)
  (set `CameraComponent.bUsePawnControlRotation` false (`/Game/Ugu/FirstPerson/Blueprints/BP_FirstPersonCharacter.FirstPersonCamera` (`self.As BP First Person Character`)))
  (set `/Game/Ugu/FirstPerson/Blueprints/BP_FirstPersonCharacter.bCanAIM` false _output_get)
  (`/Game/Ugu/FirstPerson/Blueprints/BP_FirstPersonCharacter.RecallKnife` _output_get)
  (`self.DisableInput` _returnvalue_4 _returnvalue_2)
  (`PlayerController.SetViewTargetWithBlend` _returnvalue_2 (`self.REF Camera 1`) 1.0 "VTBlend_Linear" 3.0 false)
  (bind (_outactor _returnvalue_6) (`LevelSequencePlayer.CreateLevelSequencePlayer` (`self.Cinematic1`)))
  (`MovieSceneSequencePlayer.Play` _returnvalue_6)
  (`KismetSystemLibrary.Delay` 5.6)
  (`SceneComponent.K2_SetWorldLocation` (`Actor.RootComponent` _returnvalue_5) (`self.K2_GetActorLocation` (`self.Target location Player`)) false false)
  (`SceneComponent.K2_SetWorldRotation` (`Actor.RootComponent` _returnvalue_3) (struct :`Yaw` -180.0) false false)
  (`Controller.SetControlRotation` _returnvalue (`KismetMathLibrary.FindLookAtRotation` (`self.K2_GetActorLocation` _returnvalue_5) (`self.K2_GetActorLocation` (`self.Target location camera`))))
  (`KismetSystemLibrary.Delay` 0.2)
  (set `Pawn.bUseControllerRotationYaw` true _as_bp_first_person_character)
  (set `CameraComponent.bUsePawnControlRotation` true (`/Game/Ugu/FirstPerson/Blueprints/BP_FirstPersonCharacter.FirstPersonCamera` _as_bp_first_person_character))
  (`PlayerController.SetViewTargetWithBlend` _returnvalue _returnvalue_3 0.0 "VTBlend_Linear" 3.0 false)
  (set `/Game/Ugu/FirstPerson/Blueprints/BP_FirstPersonCharacter.bCanAIM` true _as_bp_first_person_character)
  (bind _returnvalue_7 (`|CreateWidget` "/Game/Ugu/BluePrint/UI/WBP_Cladigo.WBP_Cladigo_C"))
  (bind _output_get_2 (set `self.REF_UI` _returnvalue_7))
  (`UserWidget.AddToViewport` _returnvalue_7 0)
  (`UserWidget.AddToViewport` _output_get_2 0)
  (`KismetSystemLibrary.Delay` 2.0)
  (`/Game/Ugu/BluePrint/UI/WBP_Cladigo.Input` _returnvalue_7 self))

(fn `UserConstructionScript`)