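; Pushable crate (caisse) that the first-person player can take control of and move around.
; Its box overlap registers it as the character's InteractableCaisse and shows an Interact prompt that turns to face the camera every Tick.
; While controlled, it hides the prompt, copies its stored MoveInput to the player, and snaps 200 units along the camera's forward vector, keeping its height and matching camera yaw.
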(event `self.ReceiveTick`
  (params (DeltaSeconds :type "Float (single-precision)"))
  (set `self.Delta Seconds` DeltaSeconds)
  (`self.PushCaisse`)
  (`SceneComponent.K2_SetWorldRotation` (`self.Interact`) (`KismetMathLibrary.FindLookAtRotation` (`SceneComponent.K2_GetComponentLocation` (`self.Interact`)) (`PlayerCameraManager.GetCameraLocation` (`GameplayStatics.GetPlayerCameraManager` 0))) false false))

(event `self.ReceiveBeginPlay`
  (`SceneComponent.SetVisibility` (`self.Interact`) false false))

(event `PushCaisse`
  (bind (_returnvalue_x _returnvalue_y _returnvalue_z) (`KismetMathLibrary.BreakVector` (`self.K2_GetActorLocation`)))
  (bind _returnvalue (`GameplayStatics.GetPlayerCameraManager` 0))
  (bind (_returnvalue_roll _returnvalue_pitch _returnvalue_yaw) (`KismetMathLibrary.BreakRotator` (`PlayerCameraManager.GetCameraRotation` (`GameplayStatics.GetPlayerCameraManager` 0))))
  (bind (_returnvalue_x_2 _returnvalue_y_2) (`KismetMathLibrary.BreakVector` (+ (* (`KismetMathLibrary.GetForwardVector` (`PlayerCameraManager.GetCameraRotation` _returnvalue)) 200.0) (* (`PlayerCameraManager.GetCameraLocation` _returnvalue) 1.0))))
  (if (`self.bIsControlled`)
    (set `/Game/Ugu/FirstPerson/Blueprints/BP_FirstPersonCharacter.MoveInput` (`KismetMathLibrary.MakeVector2D` (`KismetMathLibrary.BreakVector2D` (stale `SetMoveInput` _output_get)) (`.Y` (`KismetMathLibrary.BreakVector2D` (stale `SetMoveInput` _output_get)))) (`self.PlayerRef`))
    (`SceneComponent.SetVisibility` (`self.Interact`) false false)
    (`/Engine/EditorBlueprintResources/StandardMacros.IsValid` (`self.PlayerRef`)
      (:`Is Valid`
        (`self.K2_SetActorLocation` (`KismetMathLibrary.MakeVector` _returnvalue_x_2 _returnvalue_y_2 _returnvalue_z))
        (`self.K2_SetActorRotation` (`KismetMathLibrary.MakeRotator` 0.0 0.0 _returnvalue_yaw))))))

(event `StartControlCaisse`
  (set `self.bIsControlled` true))

(event `SetMoveInput`
  (params (Input :type "Vector2D Structure"))
  (bind _output_get (set `self.MoveInput` Input)))

(event `StopControlCaisse`
  (set `self.bIsControlled` false))

(event `self.Box.OnComponentBeginOverlap`
  (params (OverlappedComponent :type "PrimitiveComponent Object Reference") (OtherActor :type "Actor Object Reference") (OtherComp :type "PrimitiveComponent Object Reference") (OtherBodyIndex :type Integer) (bFromSweep :type Boolean) (SweepResult :type "HitResult Structure (by ref)"))
  (bind _asbp_first_person_character (cast `/Game/Ugu/FirstPerson/Blueprints/BP_FirstPersonCharacter` OtherActor))
  (set `/Game/Ugu/FirstPerson/Blueprints/BP_FirstPersonCharacter.InteractableCaisse` self _asbp_first_person_character)
  (set `self.PlayerRef` _asbp_first_person_character)
  (set `self.bCanInteract` true)
  (`SceneComponent.SetVisibility` (`self.Interact`) true false))

(event `self.Box.OnComponentEndOverlap`
  (params (OverlappedComponent :type "PrimitiveComponent Object Reference") (OtherActor :type "Actor Object Reference") (OtherComp :type "PrimitiveComponent Object Reference") (OtherBodyIndex :type Integer))
  (bind _asbp_first_person_character (cast `/Game/Ugu/FirstPerson/Blueprints/BP_FirstPersonCharacter` OtherActor))
  (set `/Game/Ugu/FirstPerson/Blueprints/BP_FirstPersonCharacter.InteractableCaisse` null _asbp_first_person_character)
  (set `self.PlayerRef` _asbp_first_person_character)
  (set `self.bCanInteract` false)
  (`SceneComponent.SetVisibility` (`self.Interact`) false false))

(fn `UserConstructionScript`)