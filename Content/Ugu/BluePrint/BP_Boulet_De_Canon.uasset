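; BP_Boulet_De_Canon is a cannonball the player can pick up, carry and drop, with an interact prompt shown while in reach.
; While controlled, physics is off and Tick sweeps it to a point in front of the camera, matching camera yaw.
; Release restores physics with a heavy mass scale and calls CanBreak on the first BP_Planche_Kcorp found.
; The prompt follows the ball at a fixed world height, yawed toward the camera.
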(event `self.ReceiveBeginPlay`
  (`SceneComponent.SetVisibility` (`self.Interact`) false false))

(event `self.ReceiveTick`
  (params (DeltaSeconds :type "Float (single-precision)"))
  (bind (_returnvalue_roll _returnvalue_pitch _returnvalue_yaw) (`KismetMathLibrary.BreakRotator` (`KismetMathLibrary.FindLookAtRotation` (`SceneComponent.K2_GetComponentLocation` (`self.Interact`)) (`PlayerCameraManager.GetCameraLocation` (`GameplayStatics.GetPlayerCameraManager` 0)))))
  (`self.Boulet_En_Main`)
  (`SceneComponent.K2_SetWorldLocation` (`self.Interact`) (`KismetMathLibrary.MakeVector` (.x (`self.K2_GetActorLocation`)) (.y (`self.K2_GetActorLocation`)) 60.0) false false)
  (`SceneComponent.K2_SetWorldRotation` (`self.Interact`) (`KismetMathLibrary.MakeRotator` 0.0 0.0 _returnvalue_yaw) false false))

(event `/Game/Ugu/BluePrint/BPI_Interact.CanInteract`
  (if (not (`self.bIsControlled`))
    (`SceneComponent.SetVisibility` (`self.Interact`) true false)))

(event `Boulet_En_Main`
  (bind _returnvalue (`GameplayStatics.GetPlayerCameraManager` 0))
  (bind (_returnvalue_roll _returnvalue_pitch _returnvalue_yaw) (`KismetMathLibrary.BreakRotator` (`PlayerCameraManager.GetCameraRotation` (`GameplayStatics.GetPlayerCameraManager` 0))))
  (bind (_returnvalue_x _returnvalue_y _returnvalue_z) (`KismetMathLibrary.BreakVector` (+ (* (`KismetMathLibrary.GetForwardVector` (`PlayerCameraManager.GetCameraRotation` _returnvalue)) 75.0) (* (`PlayerCameraManager.GetCameraLocation` _returnvalue) 1.0))))
  (if (`self.bIsControlled`)
    (`self.K2_SetActorLocation` (`KismetMathLibrary.MakeVector` _returnvalue_x _returnvalue_y _returnvalue_z) true)
    (`self.K2_SetActorRotation` (`KismetMathLibrary.MakeRotator` 0.0 0.0 _returnvalue_yaw))))

(event `/Game/Ugu/BluePrint/BPI_Interact.Can't Interact Object`
  (`SceneComponent.SetVisibility` (`self.Interact`) false false))

(event `StopControlBall`
  (params (Ref :type "/Game/Ugu/FirstPerson/Blueprints/BP_FirstPersonCharacter Object Reference"))
  (set `self.bIsControlled` false)
  (`PrimitiveComponent.SetSimulatePhysics` (`self.Sphere`) true)
  (`PrimitiveComponent.SetMassScale` (`self.Sphere`) "None" 100.0)
  (`SceneComponent.SetVisibility` (`self.Interact`) true false)
  (bind _outactors (`GameplayStatics.GetAllActorsOfClass` "/Game/Ugu/BluePrint/BP_Planche_Kcorp.BP_Planche_Kcorp_C"))
  (`/Game/Ugu/BluePrint/BP_Planche_Kcorp.CanBreak` (`|GetArrayItem` _outactors)))

(event `ControlBall`
  (params (Ref :type "/Game/Ugu/FirstPerson/Blueprints/BP_FirstPersonCharacter Object Reference"))
  (set `self.bIsControlled` true)
  (`PrimitiveComponent.SetSimulatePhysics` (`self.Sphere`) false)
  (`SceneComponent.SetVisibility` (`self.Interact`) false false))

(fn `UserConstructionScript`)