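; BP_CrabiCrabobo1 is an actor, apparently a crab encounter, that starts a quick-time event when the first-person character enters its box trigger.
; On overlap it reads the character's Knife flag to choose one of two QTE IDs.
; It then passes that ID and itself to the QTE manager's StartQTE, provided the manager reference is valid.
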(event `self.Box.OnComponentBeginOverlap`
  (params (OverlappedComponent :type "PrimitiveComponent Object Reference") (OtherActor :type "Actor Object Reference") (OtherComp :type "PrimitiveComponent Object Reference") (OtherBodyIndex :type Integer) (bFromSweep :type Boolean) (SweepResult :type "HitResult Structure (by ref)"))
  (bind _qtemanagerref (`self.QTEManagerRef`))
  (bind _qtemanagerref_2 (`self.QTEManagerRef`))
  (bind _asbp_first_person_character (cast `/Game/Ugu/FirstPerson/Blueprints/BP_FirstPersonCharacter` OtherActor))
  (if (`/Game/Ugu/FirstPerson/Blueprints/BP_FirstPersonCharacter.Knife?` _asbp_first_person_character)
    (set `self.QTE_ID` 1)
    (`/Engine/EditorBlueprintResources/StandardMacros.IsValid` _qtemanagerref_2
      (:`Is Valid`
        (`/Game/Ugu/BluePrint/BP_QTEManager.Start_QTE` _qtemanagerref_2 (`self.QTE_ID`) self)))
    (else
      (set `self.QTE_ID` 2)
      (`/Engine/EditorBlueprintResources/StandardMacros.IsValid` _qtemanagerref
        (:`Is Valid`
          (`/Game/Ugu/BluePrint/BP_QTEManager.Start_QTE` _qtemanagerref (`self.QTE_ID`) self))))))

(fn `UserConstructionScript`)