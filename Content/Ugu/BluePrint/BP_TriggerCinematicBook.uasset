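; BP_TriggerCinematicBook is a one-shot trigger box that plays a book-reading cinematic for the first-person character.
; On overlap it disables player input and further overlaps, blends the view to a camera and starts a level sequence.
; After delays, it shows the WBP_BookRead widget, then passes itself to that widget's Input.
; The FTG event removes the widget, blends the view back to the player and restores input.
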(event `FTG`
  (`KismetSystemLibrary.PrintString` "JAJAJAJAJA")
  (`Widget.RemoveFromParent` (`self.REF_UI`))
  (`PlayerController.SetViewTargetWithBlend` (`GameplayStatics.GetPlayerController` 0) (`GameplayStatics.GetPlayerCharacter` 0) 1.0 "VTBlend_Linear" 3.0 false)
  (`self.EnableInput` (`GameplayStatics.GetPlayerCharacter` 0) (`GameplayStatics.GetPlayerController` 0)))

(event `self.Box.OnComponentBeginOverlap`
  (params (OverlappedComponent :type "PrimitiveComponent Object Reference") (OtherActor :type "Actor Object Reference") (OtherComp :type "PrimitiveComponent Object Reference") (OtherBodyIndex :type Integer) (bFromSweep :type Boolean) (SweepResult :type "HitResult Structure (by ref)"))
  (cast `/Game/Ugu/FirstPerson/Blueprints/BP_FirstPersonCharacter` OtherActor)
  (`self.DisableInput` (`GameplayStatics.GetPlayerCharacter` 0) (`GameplayStatics.GetPlayerController` 0))
  (set `PrimitiveComponent.bGenerateOverlapEvents` false (`self.Box`))
  (`PlayerController.SetViewTargetWithBlend` (`GameplayStatics.GetPlayerController` 0) (`self.REF Camera 1`) 1.0 "VTBlend_Linear" 3.0 false)
  (bind (_outactor _returnvalue) (`LevelSequencePlayer.CreateLevelSequencePlayer` (`self.Cinematic1`)))
  (`MovieSceneSequencePlayer.Play` _returnvalue)
  (`KismetSystemLibrary.Delay` 4.0)
  (bind _returnvalue_2 (`|CreateWidget` "/Game/Ugu/BluePrint/UI/WBP_BookRead.WBP_BookRead_C"))
  (bind _output_get (set `self.REF_UI` _returnvalue_2))
  (`UserWidget.AddToViewport` _returnvalue_2 0)
  (`UserWidget.AddToViewport` _output_get 0)
  (`KismetSystemLibrary.Delay` 2.0)
  (`/Game/Ugu/BluePrint/UI/WBP_BookRead.Input` _returnvalue_2 self))

(fn `UserConstructionScript`)