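; BP_KeyDoorLockCap is a key pickup that starts hidden and unlocks a referenced door when the player touches it.
; The key mesh and its R trigger begin with collision off until the Drop_Key event reveals the mesh and enables collision and overlaps.
; When BP_FirstPersonCharacter overlaps R, it prints a pickup message and calls OpenDoorLock on the door reference, leaving the key in place.
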(event `self.ReceiveBeginPlay`
  (bind _r (`self.r`))
  (`SceneComponent.SetVisibility` (`self.polySurface1209`) false true)
  (`PrimitiveComponent.SetCollisionEnabled` _r "NoCollision")
  (`PrimitiveComponent.SetCollisionEnabled` (`self.polySurface1209`) "NoCollision")
  (set `PrimitiveComponent.bGenerateOverlapEvents` false _r))

(event `Drop_Key`
  (bind _r (`self.r`))
  (`SceneComponent.SetVisibility` (`self.polySurface1209`) true true)
  (`PrimitiveComponent.SetCollisionEnabled` _r "QueryAndPhysics")
  (`PrimitiveComponent.SetCollisionEnabled` (`self.polySurface1209`) "QueryAndPhysics")
  (set `PrimitiveComponent.bGenerateOverlapEvents` true _r))

(event `self.r.OnComponentBeginOverlap`
  (params (OverlappedComponent :type "PrimitiveComponent Object Reference") (OtherActor :type "Actor Object Reference") (OtherComp :type "PrimitiveComponent Object Reference") (OtherBodyIndex :type Integer) (bFromSweep :type Boolean) (SweepResult :type "HitResult Structure (by ref)"))
  (cast `/Game/Ugu/FirstPerson/Blueprints/BP_FirstPersonCharacter` OtherActor)
  (`KismetSystemLibrary.PrintString` "You got key")
  (`/Game/Ugu/BluePrint/BP_Door_CaptainLock.Open_Door_Lock` (`self.REF_BP_Door_CApt_Lock`)))

(fn `UserConstructionScript`)