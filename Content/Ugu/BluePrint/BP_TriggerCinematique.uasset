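; Trigger actor that plays a one-shot slow-motion cinematic when the first-person character overlaps it.
; It blends to a camera, plays a Level Sequence, then after a delay moves the player to a target, re-aims the view and restores control.
; TriggerCaleIsPast picks the variant: false disables input, removes the knife and calls the knife-stealing crab; true reveals two traps and closes a locked door.
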(event `self.Trigger.OnComponentBeginOverlap`
  (params (OverlappedComponent :type "PrimitiveComponent Object Reference") (OtherActor :type "Actor Object Reference") (OtherComp :type "PrimitiveComponent Object Reference") (OtherBodyIndex :type Integer) (bFromSweep :type Boolean) (SweepResult :type "HitResult Structure (by ref)"))
  (bind _returnvalue (`GameplayStatics.GetPlayerCharacter` 0))
  (bind _returnvalue_2 (`GameplayStatics.GetPlayerCharacter` 0))
  (bind _returnvalue_3 (`GameplayStatics.GetPlayerController` 0))
  (bind _returnvalue_4 (`GameplayStatics.GetPlayerController` 0))
  (bind _returnvalue_5 (`GameplayStatics.GetPlayerCharacter` 0))
  (bind _returnvalue_6 (`GameplayStatics.GetPlayerCharacter` 0))
  (bind _returnvalue_7 (`GameplayStatics.GetPlayerCharacter` 0))
  (bind _as_bp_first_person_character (`self.As BP First Person Character`))
  (bind _as_bp_first_person_character_2 (`self.As BP First Person Character`))
  (bind _as_bp_first_person_character_3 (`self.As BP First Person Character`))
  (bind _as_bp_first_person_character_4 (`self.As BP First Person Character`))
  (bind _returnvalue_8 (`KismetMathLibrary.FindLookAtRotation` (`self.K2_GetActorLocation` _returnvalue_7) (`self.K2_GetActorLocation` (`self.Target location camera`))))
  (bind _returnvalue_9 (`KismetMathLibrary.FindLookAtRotation` (`self.K2_GetActorLocation` _returnvalue_6) (`self.K2_GetActorLocation` (`self.Target location camera`))))
  (bind _asbp_first_person_character (cast `/Game/Ugu/FirstPerson/Blueprints/BP_FirstPersonCharacter` OtherActor))
  (bind _output_get (set `self.As BP First Person Character` _asbp_first_person_character))
  (`|ExecutionSequence`
    (:`then_0`
      (set `Pawn.bUseControllerRotationYaw` false _as_bp_first_person_character_3)
      (set `CameraComponent.bUsePawnControlRotation` false (`/Game/Ugu/FirstPerson/Blueprints/BP_FirstPersonCharacter.FirstPersonCamera` _as_bp_first_person_character_3))
      (if (not (`self.bTriggerCaleIsPast`))
        (set `PrimitiveComponent.bGenerateOverlapEvents` false (`self.Trigger`))
        (set `PrimitiveComponent.bGenerateOverlapEvents` false (`Character.CapsuleComponent` _output_get))
        (set `/Game/Ugu/FirstPerson/Blueprints/BP_FirstPersonCharacter.Knife?` false _output_get)
        (`KismetSystemLibrary.PrintString` "Plus de couteau")
        (`self.DisableInput` _returnvalue_5 (`GameplayStatics.GetPlayerController` 0))
        (`GameplayStatics.SetGlobalTimeDilation` 0.5)
        (`PlayerController.SetViewTargetWithBlend` (`GameplayStatics.GetPlayerController` 0) (`self.REF Camera 1`) 1.0 "VTBlend_Linear" 3.0 false)
        (bind (_outactor _returnvalue_10) (`LevelSequencePlayer.CreateLevelSequencePlayer` (`self.Cinematic1`)))
        (`MovieSceneSequencePlayer.Play` _returnvalue_10)
        (`KismetSystemLibrary.Delay` 4.5)
        (`SceneComponent.K2_SetWorldLocation` (`Actor.RootComponent` _returnvalue_6) (`self.K2_GetActorLocation` (`self.Target location Player`)) false false)
        (`SceneComponent.K2_SetWorldRotation` (`Actor.RootComponent` _returnvalue_5) _returnvalue_9 false false)
        (`Controller.SetControlRotation` (`GameplayStatics.GetPlayerController` 0) _returnvalue_9)
        (set `Pawn.bUseControllerRotationYaw` true _as_bp_first_person_character_4)
        (set `CameraComponent.bUsePawnControlRotation` true (`/Game/Ugu/FirstPerson/Blueprints/BP_FirstPersonCharacter.FirstPersonCamera` _as_bp_first_person_character_4))
        (`PlayerController.SetViewTargetWithBlend` _returnvalue_3 _returnvalue_2 1.0 "VTBlend_Linear" 3.0 false)
        (`self.EnableInput` _returnvalue_2 _returnvalue_3)
        (`/Game/Ugu/BluePrint/BP_Crabivole_knife.CrabivoleurDeCouteau` (`self.REF_CrabiVoleur`))
        (`GameplayStatics.SetGlobalTimeDilation` 1.0)
        (set `PrimitiveComponent.bGenerateOverlapEvents` true (`Character.CapsuleComponent` _returnvalue_2))))
    (:`then_1`
      (if (`self.bTriggerCaleIsPast`)
        (set `Pawn.bUseControllerRotationYaw` false _as_bp_first_person_character_2)
        (set `CameraComponent.bUsePawnControlRotation` false (`/Game/Ugu/FirstPerson/Blueprints/BP_FirstPersonCharacter.FirstPersonCamera` _as_bp_first_person_character_2))
        (set `PrimitiveComponent.bGenerateOverlapEvents` false (`self.Trigger`))
        (`GameplayStatics.SetGlobalTimeDilation` 0.5)
        (`PlayerController.SetViewTargetWithBlend` (`GameplayStatics.GetPlayerController` 0) (`self.REF Camera 1`) 1.0 "VTBlend_Linear" 3.0 false)
        (bind (_outactor_2 _returnvalue_11) (`LevelSequencePlayer.CreateLevelSequencePlayer` (`self.Cinematic1`)))
        (`MovieSceneSequencePlayer.Play` _returnvalue_11)
        (if (`self.bTriggerCaleIsPast`)
          (`/Game/Ugu/BluePrint/BP_Trap.Open_Visibility` (`self.REF_BP_Trap`))
          (`/Game/Ugu/BluePrint/BP_Trap_Retour.Open_Visibility_Return` (`self.Ref_BP_Trap_Retour`))
          (`/Game/Ugu/BluePrint/BP_Door_CaptainLock.Close_Door_Lock` (`self.REF_BP_DoorLock`))
          (`KismetSystemLibrary.Delay` 6.0)
          (`SceneComponent.K2_SetWorldLocation` (`Actor.RootComponent` _returnvalue_7) (`self.K2_GetActorLocation` (`self.Target location Player`)) false false)
          (`SceneComponent.K2_SetWorldRotation` (`Actor.RootComponent` _returnvalue) _returnvalue_8 false false)
          (`Controller.SetControlRotation` _returnvalue_4 _returnvalue_8)
          (set `Pawn.bUseControllerRotationYaw` true _as_bp_first_person_character)
          (set `CameraComponent.bUsePawnControlRotation` true (`/Game/Ugu/FirstPerson/Blueprints/BP_FirstPersonCharacter.FirstPersonCamera` _as_bp_first_person_character))
          (`PlayerController.SetViewTargetWithBlend` _returnvalue_4 _returnvalue 0.0 "VTBlend_Linear" 3.0 false)
          (`self.EnableInput` _returnvalue _returnvalue_4)
          (`GameplayStatics.SetGlobalTimeDilation` 1.0))))))

(fn `UserConstructionScript`)