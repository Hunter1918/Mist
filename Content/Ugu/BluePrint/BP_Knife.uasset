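; BP_Knife is a knife pickup actor with an Interact indicator that turns to face the player camera every tick.
; The indicator starts hidden, and the CanInteract and Can'tInteractObject events show or hide it while the IsValid flag is false.
; Get_Knife sets IsValid, which stops those visibility changes, then destroys the actor after a short delay.
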(event `self.ReceiveTick`
  (params (DeltaSeconds :type "Float (single-precision)"))
  (`SceneComponent.K2_SetWorldRotation` (`self.Interact`) (`KismetMathLibrary.FindLookAtRotation` (`SceneComponent.K2_GetComponentLocation` (`self.Interact`)) (`PlayerCameraManager.GetCameraLocation` (`GameplayStatics.GetPlayerCameraManager` 0))) false false))

(event `self.ReceiveBeginPlay`
  (`SceneComponent.SetVisibility` (`self.Interact`) false false))

(event `Get_Knife`
  (set `self.bIsValid` true)
  (`KismetSystemLibrary.Delay` 0.2)
  (`self.K2_DestroyActor`))

(event `/Game/Ugu/BluePrint/BPI_Interact.CanInteract`
  (if (not (`self.bIsValid`))
    (`SceneComponent.SetVisibility` (`self.Interact`) true false)))

(event `/Game/Ugu/BluePrint/BPI_Interact.Can't Interact Object`
  (if (not (`self.bIsValid`))
    (`SceneComponent.SetVisibility` (`self.Interact`) false false)))

(fn `UserConstructionScript`)