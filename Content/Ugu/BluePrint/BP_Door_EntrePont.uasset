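; Puzzle door Blueprint that swings open once when Open_Door_Puzzle fires.
; A timeline yaws the door mesh a quarter turn, guarded by the DoorOpen flag.
; An Interact indicator starts hidden, is toggled by the interaction events, and turns toward the player camera on Tick.
; Once the door is flagged open, Tick destroys the indicator and clears IsValid to stop updating it.
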(event `self.ReceiveBeginPlay`
  (`SceneComponent.SetVisibility` (`self.Interact`) false false))

(event `Open_Door_Puzzle`
  (if (not (`self.Door Open`))
    (set `self.Door Open` true)
    (bind (_direction _door_track) (`Timeline|Timeline` :!via `PlayFromStart`)
      (:`Update`
        (`SceneComponent.K2_SetRelativeRotation` (`self.polySurface275`) (`KismetMathLibrary.MakeRotator` 0.0 0.0 (`KismetMathLibrary.Lerp` 0.0 -90.0 _door_track)) false false)))))

(event `self.ReceiveTick`
  (params (DeltaSeconds :type "Float (single-precision)"))
  (if (`self.bIsValid`)
    (`SceneComponent.K2_SetWorldRotation` (`self.Interact`) (`KismetMathLibrary.FindLookAtRotation` (`SceneComponent.K2_GetComponentLocation` (`self.Interact`)) (`PlayerCameraManager.GetCameraLocation` (`GameplayStatics.GetPlayerCameraManager` 0))) false false)
    (if (`self.Door Open`)
      (`ActorComponent.K2_DestroyComponent` (`self.Interact`))
      (set `self.bIsValid` false))))

(event `/Game/Ugu/BluePrint/BPI_Interact.CanInteract`
  (`SceneComponent.SetVisibility` (`self.Interact`) true false))

(event `/Game/Ugu/BluePrint/BPI_Interact.Can't Interact Object`
  (`SceneComponent.SetVisibility` (`self.Interact`) false false))

(fn `UserConstructionScript`)