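; BP_Planche is a plank actor made of two mesh pieces that falls and dissolves away when its Drop event is called.
; Drop enables physics on both pieces and gives each a dynamic material instance.
; Two timelines, one per piece, drive the "Disolve" scalar parameter.
; Each timeline's Update also feeds a short Delay before DestroyActor, so the actor removes itself seconds after the drop.
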(event `Drop`
  (bind _polysurface280 (`self.polySurface280`))
  (bind _polysurface279 (`self.polySurface279`))
  (`PrimitiveComponent.SetSimulatePhysics` (`self.polySurface280`) true)
  (`PrimitiveComponent.SetSimulatePhysics` (`self.polySurface279`) true)
  (`|ExecutionSequence`
    (:`then_0`
      (bind _returnvalue (`PrimitiveComponent.CreateDynamicMaterialInstance` _polysurface280 0 (`PrimitiveComponent.GetMaterial` _polysurface280 0) "None"))
      (bind (_direction _newtrack_0) (`Timeline|Timeline` :!via `PlayFromStart`)
        (:`Update`
          (`MaterialInstanceDynamic.SetScalarParameterValue` _returnvalue "Disolve" _newtrack_0)
          (`KismetSystemLibrary.Delay` 3.0)
          (`self.K2_DestroyActor`))))
    (:`then_1`
      (bind _returnvalue_2 (`PrimitiveComponent.CreateDynamicMaterialInstance` _polysurface279 0 (`PrimitiveComponent.GetMaterial` _polysurface279 0) "None"))
      (bind (_direction_2 _newtrack_0_2) (`Timeline|Timeline_0` :!via `PlayFromStart`)
        (:`Update`
          (`MaterialInstanceDynamic.SetScalarParameterValue` _returnvalue_2 "Disolve" _newtrack_0_2)
          (`KismetSystemLibrary.Delay` 3.0)
          (`self.K2_DestroyActor`))))))

(fn `UserConstructionScript`)