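; Droppable crate actor that falls, dissolves and removes itself when its Drop event is called.
; Drop enables physics on the PCube7 mesh, then creates dynamic material instances for PCube7 and PCube5.
; A separate timeline drives each material's "Disolve" parameter.
; Each timeline's Update also runs into a short delay that destroys the actor, so removal is timed from the dissolve's start.
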(event `Drop`
  (bind _pcube7 (`self.pCube7`))
  (bind _pcube5 (`self.pCube5`))
  (`PrimitiveComponent.SetSimulatePhysics` (`self.pCube7`) true)
  (`|ExecutionSequence`
    (:`then_0`
      (bind _returnvalue (`PrimitiveComponent.CreateDynamicMaterialInstance` _pcube7 0 (`PrimitiveComponent.GetMaterial` _pcube7 0) "None"))
      (bind (_direction _newtrack_0) (`Timeline|Timeline` :!via `PlayFromStart`)
        (:`Update`
          (`MaterialInstanceDynamic.SetScalarParameterValue` _returnvalue "Disolve" _newtrack_0)
          (`KismetSystemLibrary.Delay` 3.0)
          (`self.K2_DestroyActor`))))
    (:`then_1`
      (bind _returnvalue_2 (`PrimitiveComponent.CreateDynamicMaterialInstance` _pcube5 0 (`PrimitiveComponent.GetMaterial` _pcube5 0) "None"))
      (bind (_direction_2 _newtrack_0_2) (`Timeline|Timeline_0` :!via `PlayFromStart`)
        (:`Update`
          (`MaterialInstanceDynamic.SetScalarParameterValue` _returnvalue_2 "Disolve" _newtrack_0_2)
          (`KismetSystemLibrary.Delay` 3.0)
          (`self.K2_DestroyActor`))))))

(fn `UserConstructionScript`)