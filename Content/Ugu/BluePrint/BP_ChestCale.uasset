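; BP_ChestCale is a one-time interactable chest with a camera-facing prompt, shown only when the character's OpenChest flag is set.
; Opening it disables input, blends to a fixed camera and spawns the WBP_Maria widget, passing itself after a delay.
; Remove_UI clears the widget, plays a level sequence, then after a timed delay repositions and re-aims the player, restoring view and input.
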(event `Remove_UI`
  (bind _returnvalue (`GameplayStatics.GetPlayerController` 0))
  (bind _returnvalue_2 (`GameplayStatics.GetPlayerCharacter` 0))
  (bind _as_bp_first_person_character (`self.As BP First Person Character`))
  (bind _asbp_first_person_character (cast `/Game/Ugu/FirstPerson/Blueprints/BP_FirstPersonCharacter` (`GameplayStatics.GetPlayerCharacter` 0)))
  (bind _output_get (set `self.As BP First Person Character` _asbp_first_person_character))
  (set `Pawn.bUseControllerRotationYaw` false _output_get)
  (set `CameraComponent.bUsePawnControlRotation` false (`/Game/Ugu/FirstPerson/Blueprints/BP_FirstPersonCharacter.FirstPersonCamera` _output_get))
  (`Widget.RemoveFromParent` (`self.REF_UI`))
  (bind (_outactor _returnvalue_3) (`LevelSequencePlayer.CreateLevelSequencePlayer` (`self.Cinematique`)))
  (`MovieSceneSequencePlayer.Play` _returnvalue_3)
  (`KismetSystemLibrary.Delay` 5.1)
  (`SceneComponent.K2_SetWorldLocation` (`Actor.RootComponent` (`GameplayStatics.GetPlayerCharacter` 0)) (`self.K2_GetActorLocation` (`self.Ref Player Location`)) false false)
  (`Controller.SetControlRotation` (`GameplayStatics.GetPlayerController` 0) (`KismetMathLibrary.FindLookAtRotation` (`self.K2_GetActorLocation` (`GameplayStatics.GetPlayerCharacter` 0)) (`self.K2_GetActorLocation` (`self.Target location camera`))))
  (`SceneComponent.K2_SetRelativeLocationAndRotation` (`Actor.RootComponent` (`self.camera_Ref`)) (6779.195312 -273.132874 956.0) (struct :`Pitch` -18.649553 :`Yaw` 49.16782 :`Roll` 0.572478) false false)
  (set `Pawn.bUseControllerRotationYaw` true _as_bp_first_person_character)
  (set `CameraComponent.bUsePawnControlRotation` true (`/Game/Ugu/FirstPerson/Blueprints/BP_FirstPersonCharacter.FirstPersonCamera` _as_bp_first_person_character))
  (`PlayerController.SetViewTargetWithBlend` _returnvalue _returnvalue_2 1.0 "VTBlend_Linear" 3.0 false)
  (`self.EnableInput` _returnvalue_2 _returnvalue))

(event `OpenChest`
  (if (not (`self.Open Chest`))
    (`self.DisableInput` (`GameplayStatics.GetPlayerCharacter` 0) (`GameplayStatics.GetPlayerController` 0))
    (set `self.bIsValid` false)
    (set `self.Open Chest` true)
    (`PlayerController.SetViewTargetWithBlend` (`GameplayStatics.GetPlayerController` 0) (`self.camera_Ref`) 1.0 "VTBlend_Linear" 3.0 false)
    (bind _returnvalue (`|CreateWidget` "/Game/Ugu/BluePrint/UI/WBP_Maria.WBP_Maria_C"))
    (bind _output_get (set `self.REF_UI` _returnvalue))
    (`UserWidget.AddToViewport` _output_get 0)
    (`KismetSystemLibrary.Delay` 2.0)
    (`/Game/Ugu/BluePrint/UI/WBP_Maria.Input` _returnvalue self)))

(event `self.ReceiveBeginPlay`
  (`SceneComponent.SetVisibility` (`self.Interact`) false false))

(event `/Game/Ugu/BluePrint/BPI_Interact.CanInteract`
  (bind _asbp_first_person_character (cast `/Game/Ugu/FirstPerson/Blueprints/BP_FirstPersonCharacter` (`GameplayStatics.GetPlayerCharacter` 0)))
  (if (`/Game/Ugu/FirstPerson/Blueprints/BP_FirstPersonCharacter.bOpenChest?` _asbp_first_person_character)
    (`SceneComponent.SetVisibility` (`self.Interact`) true false)))

(event `self.ReceiveTick`
  (params (DeltaSeconds :type "Float (single-precision)"))
  (if (`self.bIsValid`)
    (`SceneComponent.K2_SetWorldRotation` (`self.Interact`) (`KismetMathLibrary.FindLookAtRotation` (`SceneComponent.K2_GetComponentLocation` (`self.Interact`)) (`PlayerCameraManager.GetCameraLocation` (`GameplayStatics.GetPlayerCameraManager` 0))) false false)
    (if (`self.Open Chest`)
      (`ActorComponent.K2_DestroyComponent` (`self.Interact`))
      (set `self.bIsValid` false))
    (else
      (`SceneComponent.SetVisibility` (`self.Interact`) false false))))

(event `/Game/Ugu/BluePrint/BPI_Interact.Can't Interact Object`
  (`SceneComponent.SetVisibility` (`self.Interact`) false false))

(fn `UserConstructionScript`)