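; BP_Hammoc is a hammock actor that the player can cut, making it dissolve and disappear.
; Two triggers arm it when the first-person character or a BP_RopeKnife overlaps.
; Tick fires the destroy event if the armed player is cutting (printing that state for debug), or immediately after knife contact.
; A timeline drives the Disolve parameter on a dynamic material, with a delay started from its update before destroying the actor.
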(event `Destroy_Hammoc`
  (bind _hamak (`self.hamak`))
  (`|ExecutionSequence`
    (:`then_0`
      (if (`self.PeutCut?`)
        (set `self.PeutCut?` false)
        (bind _returnvalue (`PrimitiveComponent.CreateDynamicMaterialInstance` _hamak 0 (`PrimitiveComponent.GetMaterial` _hamak 0) "None" :!label _label))
        (bind (_direction _newtrack_0) (`Timeline|Timeline` :!via `PlayFromStart`)
          (:`Update`
            (`MaterialInstanceDynamic.SetScalarParameterValue` _returnvalue "Disolve" _newtrack_0)
            (`KismetSystemLibrary.Delay` 2.5)
            (`self.K2_DestroyActor`)))))
    (:`then_1`
      (if (`self.Cut_Distance`)
        (set `self.Cut_Distance` false)
        (goto _label)))))

(event `self.ReceiveTick`
  (params (DeltaSeconds :type "Float (single-precision)"))
  (`|ExecutionSequence`
    (:`then_0`
      (if (`self.PeutCut?`)
        (bind _asbp_first_person_character (cast `/Game/Ugu/FirstPerson/Blueprints/BP_FirstPersonCharacter` (`GameplayStatics.GetPlayerCharacter` 0)))
        (bind _biscuting (`/Game/Ugu/FirstPerson/Blueprints/BP_FirstPersonCharacter.bIsCuting` _asbp_first_person_character))
        (`KismetSystemLibrary.PrintString` (`KismetStringLibrary.Conv_BoolToString` _biscuting))
        (if _biscuting
          (`self.Destroy_Hammoc` :!label _label_2))))
    (:`then_1`
      (if (`self.Cut_Distance`)
        (goto _label_2)))))

(event `self.Trigger.OnComponentBeginOverlap`
  (params (OverlappedComponent :type "PrimitiveComponent Object Reference") (OtherActor :type "Actor Object Reference") (OtherComp :type "PrimitiveComponent Object Reference") (OtherBodyIndex :type Integer) (bFromSweep :type Boolean) (SweepResult :type "HitResult Structure (by ref)"))
  (`|ExecutionSequence`
    (:`then_0`
      (cast `/Game/Ugu/FirstPerson/Blueprints/BP_FirstPersonCharacter` OtherActor)
      (set `self.PeutCut?` true))
    (:`then_1`
      (cast `/Game/Ugu/BluePrint/BP_RopeKnife` OtherActor)
      (set `self.Cut_Distance` true))))

(event `self.Trigger.OnComponentEndOverlap`
  (params (OverlappedComponent :type "PrimitiveComponent Object Reference") (OtherActor :type "Actor Object Reference") (OtherComp :type "PrimitiveComponent Object Reference") (OtherBodyIndex :type Integer))
  (bind _asbp_first_person_character (cast `/Game/Ugu/FirstPerson/Blueprints/BP_FirstPersonCharacter` OtherActor))
  (set `self.PeutCut?` false)
  (set `/Game/Ugu/FirstPerson/Blueprints/BP_FirstPersonCharacter.bIsCuting` false _asbp_first_person_character))

(event `self.Trigger1.OnComponentBeginOverlap`
  (params (OverlappedComponent :type "PrimitiveComponent Object Reference") (OtherActor :type "Actor Object Reference") (OtherComp :type "PrimitiveComponent Object Reference") (OtherBodyIndex :type Integer) (bFromSweep :type Boolean) (SweepResult :type "HitResult Structure (by ref)"))
  (`|ExecutionSequence`
    (:`then_0`
      (cast `/Game/Ugu/FirstPerson/Blueprints/BP_FirstPersonCharacter` OtherActor)
      (set `self.PeutCut?` true))
    (:`then_1`
      (cast `/Game/Ugu/BluePrint/BP_RopeKnife` OtherActor)
      (set `self.Cut_Distance` true))))

(event `self.Trigger1.OnComponentEndOverlap`
  (params (OverlappedComponent :type "PrimitiveComponent Object Reference") (OtherActor :type "Actor Object Reference") (OtherComp :type "PrimitiveComponent Object Reference") (OtherBodyIndex :type Integer))
  (bind _asbp_first_person_character (cast `/Game/Ugu/FirstPerson/Blueprints/BP_FirstPersonCharacter` OtherActor))
  (set `self.PeutCut?` false)
  (set `/Game/Ugu/FirstPerson/Blueprints/BP_FirstPersonCharacter.bIsCuting` false _asbp_first_person_character))

(fn `UserConstructionScript`)