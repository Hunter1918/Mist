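; BP_Tentacule_Captain is a tentacle actor whose death releases a key.
; Its Dead_Tentacule_Pont event turns on skeletal mesh physics and calls DropKey on the referenced key.
; A timeline drives the Disolve parameter on a dynamic material of the static mesh.
; A delay hanging off the timeline's Update destroys the actor about five seconds after the dissolve starts.
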(event `Dead_Tentacule_Pont`
  (bind _staticmesh (`self.StaticMesh`))
  (`PrimitiveComponent.SetSimulatePhysics` (`self.SkeletalMesh`) true)
  (`/Game/Ugu/BluePrint/BP_KeyDoorLockCap.Drop_Key` (`self.REF_Key`))
  (bind _returnvalue (`PrimitiveComponent.CreateDynamicMaterialInstance` _staticmesh 0 (`PrimitiveComponent.GetMaterial` _staticmesh 0) "None"))
  (bind (_direction _newtrack_0) (`Timeline|Timeline` :!via `PlayFromStart`)
    (:`Update`
      (`MaterialInstanceDynamic.SetScalarParameterValue` _returnvalue "Disolve" _newtrack_0)
      (`KismetSystemLibrary.Delay` 5.0)
      (`self.K2_DestroyActor`))))

(fn `UserConstructionScript`)