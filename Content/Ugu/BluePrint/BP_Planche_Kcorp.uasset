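; Breakable plank that a cannonball knocks down, triggering a cinematic and unlocking the hold (Cale) door for the player.
; CanBreak stores a reference and opens a brief overlap window on the box.
; A cannonball hit decrements the player's ball count, drops linked crates and plank, destroys the stored reference, then hides and later removes this actor.
; If a sequence is set, the view blends to its camera, then back to the relocated player.
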(event `self.ReceiveBeginPlay`
  (set `PrimitiveComponent.bGenerateOverlapEvents` false (`self.Box`)))

(event `GrosKKKIPU`
  (`/Engine/EditorBlueprintResources/StandardMacros.IsValid` (`self.Cinematique`)
    (:`Is Valid`
      (`PlayerController.SetViewTargetWithBlend` (`GameplayStatics.GetPlayerController` 0) (`self.camera_Ref`) 1.0 "VTBlend_Linear" 3.0 false)
      (bind (_outactor _returnvalue) (`LevelSequencePlayer.CreateLevelSequencePlayer` (`self.Cinematique`)))
      (`MovieSceneSequencePlayer.Play` _returnvalue)
      (`KismetSystemLibrary.Delay` 5.1)
      (`SceneComponent.K2_SetWorldLocation` (`Actor.RootComponent` (`GameplayStatics.GetPlayerCharacter` 0)) (`self.K2_GetActorLocation` (`self.Ref_Player_Location`)) false false)
      (`PlayerController.SetViewTargetWithBlend` (`GameplayStatics.GetPlayerController` 0) (`GameplayStatics.GetPlayerCharacter` 0) 1.0 "VTBlend_Linear" 3.0 false)
      (`KismetSystemLibrary.PrintString` "Verterbre")
      (set `/Game/Ugu/FirstPerson/Blueprints/BP_FirstPersonCharacter.bCanOpenDoorCale` true (`self.As BP First Person Character`)))))

(event `CanBreak`
  (params (REF :type "Actor Object Reference"))
  (set `self.REF` REF)
  (set `PrimitiveComponent.bGenerateOverlapEvents` true (`self.Box`))
  (`KismetSystemLibrary.Delay` 2.0)
  (set `PrimitiveComponent.bGenerateOverlapEvents` false (`self.Box`)))

(event `self.Box.OnComponentBeginOverlap`
  (params (OverlappedComponent :type "PrimitiveComponent Object Reference") (OtherActor :type "Actor Object Reference") (OtherComp :type "PrimitiveComponent Object Reference") (OtherBodyIndex :type Integer) (bFromSweep :type Boolean) (SweepResult :type "HitResult Structure (by ref)"))
  (cast `/Game/Ugu/BluePrint/BP_Boulet_De_Canon` OtherActor)
  (bind _asbp_first_person_character (cast `/Game/Ugu/FirstPerson/Blueprints/BP_FirstPersonCharacter` (`GameplayStatics.GetPlayerCharacter` 0)))
  (set `self.As BP First Person Character` _asbp_first_person_character)
  (set `/Game/Ugu/FirstPerson/Blueprints/BP_FirstPersonCharacter.NbrOfBoulet` (- (`/Game/Ugu/FirstPerson/Blueprints/BP_FirstPersonCharacter.NbrOfBoulet` _asbp_first_person_character) 1) _asbp_first_person_character)
  (set `PrimitiveComponent.bGenerateOverlapEvents` false (`self.Box`))
  (`/Game/Ugu/BluePrint/BP_CaisseDrop.Drop` (`self.REF_Caisse`))
  (`/Game/Ugu/BluePrint/BP_CaisseDrop.Drop` (`self.REF_Caisse_0`))
  (`/Game/Ugu/BluePrint/BP_Planche.Drop` (`self.REF_Planche`))
  (`self.GrosKKKIPU`)
  (`self.K2_DestroyActor` (`self.REF`))
  (`SceneComponent.SetVisibility` (`self.DefaultSceneRoot`) false true)
  (`KismetSystemLibrary.Delay` 10.0)
  (`self.K2_DestroyActor`))

(fn `UserConstructionScript`)