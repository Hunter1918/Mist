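; BP_Tentacoule is a tentacle obstacle that starts a quick-time event when the first-person character enters its box trigger.
; The overlap passes a fixed QTE ID and itself to the referenced QTE manager.
; Its Dead_Tencacule event runs two timelines that drive a dissolve parameter on dynamic materials for the Tentacoule and E components.
; The actor is destroyed through a three-second delay triggered from the timeline updates.
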(event `Dead_Tencacule`
  (bind _tentacoule (`self.Tentacoule`))
  (bind _e (`self.e`))
  (`|ExecutionSequence`
    (:`then_0`
      (bind _returnvalue (`PrimitiveComponent.CreateDynamicMaterialInstance` _tentacoule 0 (`PrimitiveComponent.GetMaterial` _tentacoule 0) "None"))
      (bind (_direction _newtrack_0) (`Timeline|Timeline` :!via `PlayFromStart`)
        (:`Update`
          (`MaterialInstanceDynamic.SetScalarParameterValue` _returnvalue "Disolve" _newtrack_0)
          (`KismetSystemLibrary.Delay` 3.0)
          (`self.K2_DestroyActor`))))
    (:`then_1`
      (bind _returnvalue_2 (`PrimitiveComponent.CreateDynamicMaterialInstance` _e 0 (`PrimitiveComponent.GetMaterial` _e 0) "None"))
      (bind (_direction_2 _newtrack_0_2) (`Timeline|Timeline_0` :!via `PlayFromStart`)
        (:`Update`
          (`MaterialInstanceDynamic.SetScalarParameterValue` _returnvalue_2 "Disolve" _newtrack_0_2)
          (`KismetSystemLibrary.Delay` 3.0)
          (`self.K2_DestroyActor`))))))

(event `self.Box.OnComponentBeginOverlap`
  (params (OverlappedComponent :type "PrimitiveComponent Object Reference") (OtherActor :type "Actor Object Reference") (OtherComp :type "PrimitiveComponent Object Reference") (OtherBodyIndex :type Integer) (bFromSweep :type Boolean) (SweepResult :type "HitResult Structure (by ref)"))
  (bind _qtemanagerref (`self.QTEManagerRef`))
  (cast `/Game/Ugu/FirstPerson/Blueprints/BP_FirstPersonCharacter` OtherActor)
  (set `self.QTE_ID` 4)
  (`/Engine/EditorBlueprintResources/StandardMacros.IsValid` _qtemanagerref
    (:`Is Valid`
      (`/Game/Ugu/BluePrint/BP_QTEManager.Start_QTE` _qtemanagerref (`self.QTE_ID`) self))))

(fn `UserConstructionScript`)