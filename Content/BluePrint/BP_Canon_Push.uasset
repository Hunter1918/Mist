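; Pushable cannon actor that the first-person character can take control of, move around and fire.
; An interaction box registers it as the character's interactable on overlap and clears it on exit, printing debug prompts.
; While controlled, each Tick teleports it ahead of the player camera at its own height, matching camera yaw.
; Firing spawns a cannonball at the fire point behind a brief cooldown; move input is stored but unused here.
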(event `PushCanon`
  (bind (_returnvalue_x _returnvalue_y _returnvalue_z) (`KismetMathLibrary.BreakVector` (`self.K2_GetActorLocation`)))
  (bind _returnvalue (`GameplayStatics.GetPlayerCameraManager` 0))
  (bind (_returnvalue_roll _returnvalue_pitch _returnvalue_yaw) (`KismetMathLibrary.BreakRotator` (`PlayerCameraManager.GetCameraRotation` (`GameplayStatics.GetPlayerCameraManager` 0))))
  (bind (_returnvalue_x_2 _returnvalue_y_2) (`KismetMathLibrary.BreakVector` (+ (* (`KismetMathLibrary.GetForwardVector` (`PlayerCameraManager.GetCameraRotation` _returnvalue)) 200.0) (* (`PlayerCameraManager.GetCameraLocation` _returnvalue) 1.0))))
  (if (`self.bIsControlled`)
    (`/Engine/EditorBlueprintResources/StandardMacros.IsValid` (`self.PlayerRef`)
      (:`Is Valid`
        (`self.K2_SetActorLocation` (`KismetMathLibrary.MakeVector` _returnvalue_x_2 _returnvalue_y_2 _returnvalue_z) false true)
        (`self.K2_SetActorRotation` (`KismetMathLibrary.MakeRotator` 0.0 0.0 _returnvalue_yaw))))))

(event `StartControl`
  (set `self.bIsControlled` true))

(event `FireCannon`
  (if (`self.CanFire`)
    (set `self.CanFire` false)
    (`|SpawnActorFromClass` (`self.CannonBallClass`) (`SceneComponent.K2_GetComponentToWorld` (`self.FirePoint`)) "Undefined" "MultiplyWithRoot" null null)
    (`KismetSystemLibrary.Delay` 0.1)
    (set `self.CanFire` true)))

(event `SetMoveInput`
  (params (Input :type "Vector2D Structure"))
  (set `self.MoveInput` Input))

(event `StopControl`
  (set `self.bIsControlled` false))

(event `self.ReceiveTick`
  (params (DeltaSeconds :type "Float (single-precision)"))
  (set `self.Delta Seconds` DeltaSeconds)
  (`self.PushCanon`))

(event `self.BoxCollision_Interaction.OnComponentBeginOverlap`
  (params (OverlappedComponent :type "PrimitiveComponent Object Reference") (OtherActor :type "Actor Object Reference") (OtherComp :type "PrimitiveComponent Object Reference") (OtherBodyIndex :type Integer) (bFromSweep :type Boolean) (SweepResult :type "HitResult Structure (by ref)"))
  (bind _asbp_first_person_character (cast `/Game/FirstPerson/Blueprints/BP_FirstPersonCharacter` OtherActor))
  (set `/Game/FirstPerson/Blueprints/BP_FirstPersonCharacter.InteractableActor` self _asbp_first_person_character)
  (set `self.PlayerRef` _asbp_first_person_character)
  (set `self.bCanInteract` true)
  (`KismetSystemLibrary.PrintString` "Utiliser Le Canon appuie sur E la ptn de ta race nan mais SERIEUX mais que fait mon teamate (coup d'accoudoir)"))

(event `self.BoxCollision_Interaction.OnComponentEndOverlap`
  (params (OverlappedComponent :type "PrimitiveComponent Object Reference") (OtherActor :type "Actor Object Reference") (OtherComp :type "PrimitiveComponent Object Reference") (OtherBodyIndex :type Integer))
  (bind _asbp_first_person_character (cast `/Game/FirstPerson/Blueprints/BP_FirstPersonCharacter` OtherActor))
  (set `/Game/FirstPerson/Blueprints/BP_FirstPersonCharacter.InteractableActor` null _asbp_first_person_character)
  (set `self.PlayerRef` _asbp_first_person_character)
  (set `self.bCanInteract` false)
  (`KismetSystemLibrary.PrintString` "Cache moi le texte mais SERIEUX INVITE PK IL INVITE JAMAIIIIIIIIIIIIIIIIIS"))

(event `/Game/BluePrint/BPI_Interact.CanInteract`
  (`KismetSystemLibrary.PrintString` "AJSFHIVSFS")
  (`SceneComponent.SetVisibility` (`self.Interact`) true false))

(fn `UserConstructionScript`)