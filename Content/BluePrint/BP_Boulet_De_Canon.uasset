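; BP_Boulet_De_Canon is a cannonball actor that can be held in front of the player camera and released.
; ControlBall disables sphere physics and sets IsControlled; StopControlBall clears it, re-enables physics and raises the mass scale.
; While controlled, the tick-driven hold logic sweeps the actor to a fixed distance along the camera's forward vector, matching only the camera's yaw.
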(event `self.ReceiveTick`
  (params (DeltaSeconds :type "Float (single-precision)"))
  (`self.Boulet_En_Main`))

(event `Boulet_En_Main`
  (bind _returnvalue (`GameplayStatics.GetPlayerCameraManager` 0))
  (bind (_returnvalue_roll _returnvalue_pitch _returnvalue_yaw) (`KismetMathLibrary.BreakRotator` (`PlayerCameraManager.GetCameraRotation` (`GameplayStatics.GetPlayerCameraManager` 0))))
  (bind (_returnvalue_x _returnvalue_y _returnvalue_z) (`KismetMathLibrary.BreakVector` (+ (* (`KismetMathLibrary.GetForwardVector` (`PlayerCameraManager.GetCameraRotation` _returnvalue)) 200.0) (* (`PlayerCameraManager.GetCameraLocation` _returnvalue) 1.0))))
  (if (`self.bIsControlled`)
    (`self.K2_SetActorLocation` (`KismetMathLibrary.MakeVector` _returnvalue_x _returnvalue_y _returnvalue_z) true)
    (`self.K2_SetActorRotation` (`KismetMathLibrary.MakeRotator` 0.0 0.0 _returnvalue_yaw))))

(event `StopControlBall`
  (set `self.bIsControlled` false)
  (`PrimitiveComponent.SetSimulatePhysics` (`self.Sphere`) true)
  (`PrimitiveComponent.SetMassScale` (`self.Sphere`) "None" 10.0))

(event `ControlBall`
  (set `self.bIsControlled` true)
  (`PrimitiveComponent.SetSimulatePhysics` (`self.Sphere`) false))

(fn `UserConstructionScript`)