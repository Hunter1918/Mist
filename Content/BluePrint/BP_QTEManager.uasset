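; Quick-time event manager that runs timed key-press challenges selected by ID, with only QTE 1 implemented beyond a debug print.
; QTE 1 blends to a spawned fixed camera, waits randomly, then prompts for G within a short window.
; Pressing that key in the window succeeds; early presses or timeouts fail, and either outcome blends back to the player.
; A second camera event exists but is not called here.
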(event `Key|AnyKey`
  (params (Key :type "Key Structure"))
  (:`Pressed`
    (if (== Key (`self.QTEKey`))
      (if (and (`self.IsQTEActive`) (`self.CanPress`))
        (`KismetSystemLibrary.PrintString` "Succes")
        (set `self.QTESuccess` true)
        (set `self.IsQTEActive` false)
        (set `self.CanPress` false)
        (else
          (`KismetSystemLibrary.PrintString` "Fail")
          (set `self.QTESuccess` false)
          (set `self.IsQTEActive` false)
          (set `self.CanPress` false)))
      (`PlayerController.SetViewTargetWithBlend` (`GameplayStatics.GetPlayerController` 0) (`GameplayStatics.GetPlayerCharacter` 0) 1.0 "VTBlend_Linear" 3.0 false :!label _label))))

(event `Start_QTE`
  (params (QTE_ID :type Integer))
  (bind _qtetimewindow (`self.QTETimeWindow`))
  (set `self.IsQTEActive` true)
  (set `self.CanPress` false)
  (switch `int` QTE_ID
    (:`1`
      (`KismetSystemLibrary.PrintString` "QTE 1")
      (`self.CameraQTE`)
      (`self.EnableInput` (`GameplayStatics.GetPlayerCharacter` 0) (`GameplayStatics.GetPlayerController` 0))
      (set `self.QTEKey` "G")
      (set `self.QTETimeWindow` 1.0)
      (`KismetSystemLibrary.Delay` (`KismetMathLibrary.RandomFloatInRange` 1.0 3.0))
      (if (not (`self.QTESuccess`))
        (set `self.CanPress` true)
        (`KismetSystemLibrary.PrintString` "Appuyer sur G" true true (struct :`R` 0.322075 :`G` 1.0 :`B` 0.659893 :`A` 1.0) _qtetimewindow)
        (`KismetSystemLibrary.Delay` _qtetimewindow)
        (if (`self.IsQTEActive`)
          (`KismetSystemLibrary.PrintString` "Fail")
          (set `self.IsQTEActive` false)
          (set `self.CanPress` false)
          (goto _label))))
    (:`2`
      (`KismetSystemLibrary.PrintString` "QTE 2"))
    (:`3`
      (`KismetSystemLibrary.PrintString` "QTE 3"))))

(event `CameraQTE`
  (bind _returnvalue (`self.K2_GetActorLocation` (`GameplayStatics.GetPlayerCharacter` 0)))
  (bind _returnvalue_2 (`|SpawnActorFromClass` "/Game/BluePrint/BP_Camera_QTE.BP_Camera_QTE_C" (`KismetMathLibrary.MakeTransform` _returnvalue (`KismetMathLibrary.Conv_VectorToRotator` _returnvalue)) "Undefined" "MultiplyWithRoot" null null))
  (`PlayerController.SetViewTargetWithBlend` (`GameplayStatics.GetPlayerController` 0) _returnvalue_2 1.0 "VTBlend_Linear" 3.0 false)
  (`self.K2_SetActorLocationAndRotation` _returnvalue_2 (-924.693201 239.774318 205.298744) (struct :`Pitch` -22.0 :`Yaw` -150.0) false false))

(event `CameraQTE2`
  (bind _returnvalue (`self.K2_GetActorLocation` (`GameplayStatics.GetPlayerCharacter` 0)))
  (bind _returnvalue_2 (`|SpawnActorFromClass` "/Game/BluePrint/BP_Camera_QTE.BP_Camera_QTE_C" (`KismetMathLibrary.MakeTransform` _returnvalue (`KismetMathLibrary.Conv_VectorToRotator` _returnvalue)) "Undefined" "MultiplyWithRoot" null null))
  (`self.K2_SetActorLocationAndRotation` _returnvalue_2 _returnvalue (struct :`Pitch` -20.0) false false)
  (`PlayerController.SetViewTargetWithBlend` (`GameplayStatics.GetPlayerController` 0) _returnvalue_2 1.0 "VTBlend_Linear" 3.0 false))

(fn `UserConstructionScript`)